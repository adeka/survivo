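; TalkableCharacter is an NPC that the player character can start a conversation with.
; Overlapping its TalkTrigger shows a Highlight and registers it as the ThirdPersonCharacter's NearbyTalkableCharacter; leaving reverses both.
; TalkToCharacter stores the talker, creates a ConversationHUD bound to this NPC, and sets it as that character's ActiveConversation.
; CompleteConversation is an empty stub.
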(event Custom|OnComponentBeginOverlap_Event_0
  (params (OverlappedComponent :type Primitive%20Component%20Object%20Reference) (OtherActor :type Actor%20Object%20Reference) (OtherComp :type Primitive%20Component%20Object%20Reference) (OtherBodyIndex :type Integer) (bFromSweep :type Boolean) (SweepResult :type Hit%20Result%20Structure%20%28by%20ref%29))
  (bind _asthird_person_character (Utilities|Casting|CastToThirdPersonCharacter OtherActor))
  (Rendering|SetVisibility (Variables|Default|GetHighlight) true false)
  (Variables|/Game/Blueprints/Characters/ThirdPersonCharacter.ThirdPersonCharacter_C|SetNearbyTalkableCharacter _asthird_person_character self))

(event Custom|OnComponentEndOverlap_Event_0
  (params (OverlappedComponent :type Primitive%20Component%20Object%20Reference) (OtherActor :type Actor%20Object%20Reference) (OtherComp :type Primitive%20Component%20Object%20Reference) (OtherBodyIndex :type Integer))
  (bind _asthird_person_character (Utilities|Casting|CastToThirdPersonCharacter OtherActor))
  (Rendering|SetVisibility (Variables|Default|GetHighlight) false false)
  (Variables|/Game/Blueprints/Characters/ThirdPersonCharacter.ThirdPersonCharacter_C|SetNearbyTalkableCharacter _asthird_person_character 0))

(event EventBeginPlay
  (bind _talktrigger (Variables|Default|GetTalkTrigger))
  (|CallParentFunction)
  (Collision|AssignOnComponentBeginOverlap _talktrigger (delegate Custom|OnComponentBeginOverlap_Event_0))
  (Collision|AssignOnComponentEndOverlap _talktrigger (delegate Custom|OnComponentEndOverlap_Event_0)))

(fn ConstructionScript
  (|CallParentFunction)
  (Rendering|SetVisibility (Variables|Default|GetHighlight) false false))

(fn TalktoCharacter
  (params (character :type Third%20Person%20Character%20Object%20Reference))
  (bind _output_get (Variables|Default|SetTalking%20To character))
  (bind _asplayer_controller (Utilities|Casting|CastToPlayerController (Pawn|GetController _output_get)))
  (bind _returnvalue (UserInterface|CreateWidget "/Game/HUD/ConversationHUD.ConversationHUD_C" _asplayer_controller self))
  (UserInterface|Viewport|AddtoViewport _returnvalue 0)
  (Variables|/Game/Blueprints/Characters/ThirdPersonCharacter.ThirdPersonCharacter_C|SetActive%20Conversation _output_get _returnvalue)
  (return))

(fn CompleteConversation
  (return))