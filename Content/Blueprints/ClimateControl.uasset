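; Climate controller actor that transitions wind and rain intensity through sun and rain toggle inputs.
; On BeginPlay it spawns a gusting directional wind source and seeds the ClimateParams material parameter collection.
; Each input plays its own timeline, feeding one strength value into particle parameters, wind strength, the collection and rain post-process blend weight.
; Without authority, Tick keeps the root over player 0 at fixed height.
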(event EventBeginPlay
  (CallFunction|SetupWind)
  (Rendering|Material|SetScalarParameterValue "/Game/Materials/ClimateParams.ClimateParams" "Rain" 1e+01 :!class /Script/Engine.KismetMaterialLibrary)
  (Rendering|Material|SetScalarParameterValue "/Game/Materials/ClimateParams.ClimateParams" "Wind" 1e+01 :!class /Script/Engine.KismetMaterialLibrary))

(event EventTick
  (params (DeltaSeconds :type Float%20%28single-precision%29))
  (bind _returnvalue (Game|GetPlayerCharacter 0))
  (bind _returnvalue_2 (Transformation|GetActorLocation _returnvalue))
  (bind (_x _y) (Math|Vector|BreakVector _returnvalue_2))
  (Networking|SwitchHasAuthority
    (:Remote
      (Transformation|SetWorldLocation (Variables|Default|GetSharedRoot) (Math|Vector|MakeVector _x _y 33.0) false false))))

(event Input|ActionEvents|InputActionToggleSun
  (params (Key :type Key%20Structure))
  (:Pressed
    (bind _newtrack_0 (Timeline|Timeline_0 PlayFromStart)
      (:Update
        (CallFunction|SetWindandRain _newtrack_0)))))

(event Input|ActionEvents|InputActionToggleRain
  (params (Key :type Key%20Structure))
  (:Pressed
    (bind _newtrack_0 (Timeline|Timeline_1 PlayFromStart)
      (:Update
        (CallFunction|SetWindandRain _newtrack_0)))))

(fn ConstructionScript)

(fn SetupWind
  (bind _returnvalue (Game|SpawnActorfromClass "/Script/Engine.WindDirectionalSource" (Transformation|GetWorldTransform (Variables|Default|GetSharedRoot)) "AlwaysSpawn" 0 0))
  (Class|WindDirectionalSourceComponent|SetStrength (Variables|/Script/Engine.WindDirectionalSource|GetComponent _returnvalue) 1.0)
  (Control|SetRadius (Variables|/Script/Engine.WindDirectionalSource|GetComponent _returnvalue) 3e+03 :!class /Script/Engine.WindDirectionalSourceComponent)
  (Class|WindDirectionalSourceComponent|SetSpeed (Variables|/Script/Engine.WindDirectionalSource|GetComponent _returnvalue) 3.0)
  (Class|WindDirectionalSourceComponent|SetMinimumGustAmount (Variables|/Script/Engine.WindDirectionalSource|GetComponent _returnvalue) 0.0)
  (Class|WindDirectionalSourceComponent|SetMaximumGustAmount (Variables|/Script/Engine.WindDirectionalSource|GetComponent _returnvalue) 5e+01)
  (Transformation|SetWorldRotation (Variables|/Script/Engine.WindDirectionalSource|GetComponent _returnvalue) "0,-90.000000, 0" false false)
  (Variables|Default|Setwind (Variables|/Script/Engine.WindDirectionalSource|GetComponent _returnvalue))
  (return))

(fn SetWindandRain
  (params (strength_in :type Float%20%28single-precision%29))
  (LocalVariables|Setstrength strength_in)
  (Effects|Components|ParticleSystem|SetFloatParameter (Variables|Default|GetWind1) "WindIntensity" (LocalVariables|Getstrength))
  (Effects|Components|ParticleSystem|SetFloatParameter (Variables|Default|GetRain) "RainIntensity" (* (LocalVariables|Getstrength) 4e+01))
  (Class|WindDirectionalSourceComponent|SetStrength (Variables|Default|Getwind) (/ (LocalVariables|Getstrength) 1e+01))
  (Rendering|Material|SetScalarParameterValue "/Game/Materials/ClimateParams.ClimateParams" "Rain" (LocalVariables|Getstrength) :!class /Script/Engine.KismetMaterialLibrary)
  (Rendering|Material|SetScalarParameterValue "/Game/Materials/ClimateParams.ClimateParams" "Wind" (LocalVariables|Getstrength) :!class /Script/Engine.KismetMaterialLibrary)
  (Variables|/Script/Engine.PostProcessComponent|SetBlendWeight (Variables|Default|GetRainPostProcess) (/ (LocalVariables|Getstrength) 1e+01)))