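; TalkableCharacter is a character the player can talk to, where talking currently just swaps the passed Character's first mesh material to Earth.
; TalkTrigger overlaps with a ThirdPersonCharacter toggle the Highlight, hidden by default, and set or clear that player's NearbyTalkableCharacter reference.
; TalkTo proceeds only with authority, passing through ServerTalkTo to TalkToCharacter, which applies the material change.
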(event Custom|OnComponentBeginOverlap_Event_0
  (params (OverlappedComponent :type Primitive%20Component%20Object%20Reference) (OtherActor :type Actor%20Object%20Reference) (OtherComp :type Primitive%20Component%20Object%20Reference) (OtherBodyIndex :type Integer) (bFromSweep :type Boolean) (SweepResult :type Hit%20Result%20Structure%20%28by%20ref%29))
  (bind _asthird_person_character (Utilities|Casting|CastToThirdPersonCharacter OtherActor))
  (Rendering|SetVisibility (Variables|Default|GetHighlight) true false)
  (Variables|/Game/Blueprints/ThirdPersonCharacter.ThirdPersonCharacter_C|SetNearbyTalkableCharacter _asthird_person_character self))

(event Custom|Server%20TalkTo
  (params (Character :type Third%20Person%20Character%20Object%20Reference))
  (CallFunction|TalktoCharacter Character))

(event Custom|OnComponentEndOverlap_Event_0
  (params (OverlappedComponent :type Primitive%20Component%20Object%20Reference) (OtherActor :type Actor%20Object%20Reference) (OtherComp :type Primitive%20Component%20Object%20Reference) (OtherBodyIndex :type Integer))
  (bind _asthird_person_character (Utilities|Casting|CastToThirdPersonCharacter OtherActor))
  (Rendering|SetVisibility (Variables|Default|GetHighlight) false false)
  (Variables|/Game/Blueprints/ThirdPersonCharacter.ThirdPersonCharacter_C|SetNearbyTalkableCharacter _asthird_person_character 0))

(event Custom|TalkTo
  (params (Character :type Third%20Person%20Character%20Object%20Reference))
  (Networking|SwitchHasAuthority
    (:Authority
      (CallFunction|ServerTalkto Character))))

(event EventBeginPlay
  (bind _talktrigger (Variables|Default|GetTalkTrigger))
  (|CallParentFunction)
  (Collision|AssignOnComponentBeginOverlap _talktrigger (delegate Custom|OnComponentBeginOverlap_Event_0))
  (Collision|AssignOnComponentEndOverlap _talktrigger (delegate Custom|OnComponentEndOverlap_Event_0)))

(fn ConstructionScript
  (|CallParentFunction)
  (Rendering|SetVisibility (Variables|Default|GetHighlight) false false))

(fn TalktoCharacter
  (params (Character :type Third%20Person%20Character%20Object%20Reference))
  (Rendering|Material|SetMaterial (Variables|/Script/Engine.Character|GetMesh Character) 0 "/Game/Geometry/Stuff/Earth.Earth")
  (return))