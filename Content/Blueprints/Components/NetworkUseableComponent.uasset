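; NetworkUseableComponent is an actor, designed to sit under a parent actor, that makes that parent usable by players in multiplayer.
; On authority, while enabled, overlap events set or clear the parent as the ThirdPersonCharacter's OverlappingNetworkedUseable and multicast a PaperSprite highlight toggle.
; Its Use event, also authority-only, forwards the user to the parent's TriggerUseMessage if the parent implements the NetworkedUseable interface.
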(event Custom|Use
  (params (User :type Third%20Person%20Character%20Object%20Reference))
  (bind _returnvalue (Actor|GetParentActor))
  (Networking|SwitchHasAuthority
    (:Authority
      (if (Utilities|DoesObjectImplementInterface _returnvalue "/Game/Blueprints/Components/NetworkedUseable.NetworkedUseable_C")
        (Class|NetworkedUseable|TriggerUse(Message) _returnvalue User)))))

(event Custom|Multicast%20Toggle%20Highlight
  (params (bNewVisibility :type Boolean))
  (CallFunction|ToggleHighlight bNewVisibility))

(event Collision|EventActorBeginOverlap
  (params (OtherActor :type Actor%20Object%20Reference))
  ;[1 1 1] Overlapping
  (Networking|SwitchHasAuthority
    (:Authority
      (if (Variables|Default|GetEnabled)
        (bind _asthird_person_character (Utilities|Casting|CastToThirdPersonCharacter OtherActor))
        (Variables|/Game/Blueprints/Characters/ThirdPersonCharacter.ThirdPersonCharacter_C|SetOverlapping%20Networked%20Useable _asthird_person_character (Actor|GetParentActor))
        (CallFunction|MulticastToggleHighlight true)))))

(event Collision|EventActorEndOverlap
  (params (OtherActor :type Actor%20Object%20Reference))
  ;[1 1 1] Overlapping
  (Networking|SwitchHasAuthority
    (:Authority
      (if (Variables|Default|GetEnabled)
        (bind _asthird_person_character (Utilities|Casting|CastToThirdPersonCharacter OtherActor))
        (Variables|/Game/Blueprints/Characters/ThirdPersonCharacter.ThirdPersonCharacter_C|SetOverlapping%20Networked%20Useable _asthird_person_character 0)
        (CallFunction|MulticastToggleHighlight false)))))

(fn ConstructionScript)

(fn ToggleHighlight
  (params (bNewVisibility :type Boolean))
  (Rendering|SetVisibility (Variables|Default|GetPaperSprite) bNewVisibility true)
  (return))