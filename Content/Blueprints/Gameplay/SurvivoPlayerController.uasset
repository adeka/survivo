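; Player controller for a survival game that bridges UI and server actions for flag placement, clan setup and crafting.
; Owner-prefixed events create viewport widgets for flag setup, clan door passcode entry and a workbench fed by the player's known recipes.
; Server-prefixed events finish flag and house setup on a pole stand, or set up a clan on the controlled character and swing its door.
; The RecipesKnown RepNotify is empty.
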(event Custom|Owner%20Show%20SetupFlag%20HUD
  (params (PoleStand :type Pole%20Stand%20Object%20Reference))
  (bind _returnvalue (UserInterface|CreateWidget "/Game/HUD/SetupFlag.SetupFlag_C" 0 PoleStand))
  (UserInterface|Viewport|AddtoViewport _returnvalue 0))

(event Custom|Owner%20Show%20WorkbenchHUD
  (bind _returnvalue (UserInterface|CreateWidget "/Game/HUD/WorkbenchHUD.WorkbenchHUD_C" self (Variables|Default|GetRecipes%20Known)))
  (UserInterface|Viewport|AddtoViewport _returnvalue 0))

(event Custom|Owner%20Show%20ClanDoorPasscode%20HUD
  (params (ClanDoor :type Clan%20Door%20Object%20Reference))
  (bind _returnvalue (UserInterface|CreateWidget "/Game/HUD/ClanDoorPasscode.ClanDoorPasscode_C" 0 ClanDoor))
  (UserInterface|Viewport|AddtoViewport _returnvalue 0))

(event Custom|Server%20Setup%20Clan
  (params (Clan%20Name :type String) (Passcode :type String) (ClanDoor :type Clan%20Door%20Object%20Reference))
  (bind _asthird_person_character (Utilities|Casting|CastToThirdPersonCharacter (Pawn|GetControlledPawn)))
  (Default|SetupClan _asthird_person_character Clan%20Name Passcode)
  (Default|SwingDoor ClanDoor))

(event Custom|Server%20Complete%20Flag%20Setup
  (params (PoleStand :type Pole%20Stand%20Object%20Reference) (Flag%20Text :type String) (Character :type Third%20Person%20Character%20Object%20Reference) (Passcode :type String))
  (Default|SetupFlagandHouse PoleStand Character Character Flag%20Text Passcode))

(event EventBeginPlay)

(event EventTick
  (params (DeltaSeconds :type Float%20%28single-precision%29)))

(fn ConstructionScript)

(fn OnRepRecipesKnown)