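; Equippable item Blueprint that toggles itself as equipment on the character that uses it.
; UseEquippable checks for network authority and only then calls ServerUseEquippable, which passes the item to the character's ToggleEquipment.
; A use on a non-authority instance does nothing, and the equip logic itself lives on the character.
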(event Custom|Use%20Equippable
  (params (character :type Third%20Person%20Character%20Object%20Reference))
  ;[1 1 1] Use Equippable
  (Networking|SwitchHasAuthority
    (:Authority
      (CallFunction|ServerUseEquippable character))))

(event Custom|Server%20Use%20Equippable
  (params (character :type Third%20Person%20Character%20Object%20Reference))
  ;[1 1 1] Use Equippable
  (Default|ToggleEquipment character self))

(event EventBeginPlay
  (|CallParentFunction))

(event Collision|EventActorBeginOverlap
  (params (OtherActor :type Actor%20Object%20Reference))
  (|CallParentFunction OtherActor))

(event EventTick
  (params (DeltaSeconds :type Float%20%28single-precision%29))
  (|CallParentFunction DeltaSeconds))

(fn ConstructionScript
  (|CallParentFunction))