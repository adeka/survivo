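; Base pickupable item actor that a character adds to itself when used.
; TriggerUse runs only with authority, forwarding to a server event that calls the character's PickupItem with this actor.
; A multicast event then hides the root and its children and disables further use, leaving the actor in the world rather than destroying it.
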(event Custom|Server%20Trigger%20Use
  (params (character :type Third%20Person%20Character%20Object%20Reference))
  (bind _self self)
  ;[1 1 1] Trigger Use
  (Default|PickupItem character _self)
  (CallFunction|MulticastUseItem _self character))

(event Custom|Multicast%20Use%20Item
  (params (Character :type Third%20Person%20Character%20Object%20Reference))
  ;[1 1 1] Multicasted Use ITem
  (Rendering|SetVisibility (Variables|Default|GetDefaultSceneRoot) false true)
  (CallFunction|DisableUse))

(event EventBeginPlay
  (|CallParentFunction))

(event Collision|EventActorBeginOverlap
  (params (OtherActor :type Actor%20Object%20Reference))
  (|CallParentFunction OtherActor))

(event EventTick
  (params (DeltaSeconds :type Float%20%28single-precision%29))
  (|CallParentFunction DeltaSeconds))

(event EventTriggerUse
  (params (character :type Third%20Person%20Character%20Object%20Reference))
  ;[1 1 1] Trigger Use
  (Networking|SwitchHasAuthority
    (:Authority
      (CallFunction|ServerTriggerUse character))))

(fn ConstructionScript
  (|CallParentFunction))