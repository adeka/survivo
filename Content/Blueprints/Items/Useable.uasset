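; Useable is a base actor for items the player can interact with in the world.
; While Enabled, overlapping a ThirdPersonCharacter sets itself as that character's OverlappingPickup and shows the Highlight component, clearing both when the overlap ends.
; TriggerUse is an empty hook, presumably for child items to override, and DisableUse turns off Enabled and hides the highlight.
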(event Collision|EventActorBeginOverlap
  (params (OtherActor :type Actor%20Object%20Reference))
  ;[1 1 1] Overlap Begin
  (if (Variables|Default|GetEnabled)
    (bind _asthird_person_character (Utilities|Casting|CastToThirdPersonCharacter OtherActor))
    (Variables|/Game/Blueprints/Characters/ThirdPersonCharacter.ThirdPersonCharacter_C|SetoverlappingPickup _asthird_person_character self)
    (CallFunction|ToggleHighlight true)))

(event Collision|EventActorEndOverlap
  (params (OtherActor :type Actor%20Object%20Reference))
  ;[1 1 1] Overlap End
  (if (Variables|Default|GetEnabled)
    (bind _asthird_person_character (Utilities|Casting|CastToThirdPersonCharacter OtherActor))
    (Variables|/Game/Blueprints/Characters/ThirdPersonCharacter.ThirdPersonCharacter_C|SetoverlappingPickup _asthird_person_character 0)
    (CallFunction|ToggleHighlight false)))

(fn ConstructionScript
  (Rendering|SetVisibility (Variables|Default|Gethighlight) false false))

(fn ToggleHighlight
  (params (toggle :type Boolean))
  (Rendering|SetVisibility (Variables|Default|Gethighlight) toggle false)
  (return))

(fn TriggerUse
  (params (character :type Third%20Person%20Character%20Object%20Reference))
  (return))

(fn DisableUse
  (Variables|Default|SetEnabled false)
  (CallFunction|ToggleHighlight false)
  (return))