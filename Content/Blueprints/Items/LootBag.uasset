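; LootBag is a networked physical bag actor that stores resource counts, grows as items are added and can be leashed to a player.
; A server event adds items (only Logs are counted, as wood), then multicasts a mass and scale update from the total.
; Leashing spawns a physics-constraint actor linking mesh to player capsule and multicasts the cable attachment; detach is empty.
; Removal spends wood only, destroying the bag when wood runs out.
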(event Custom|Server%20Add%20Item%20to%20Inventory
  (params (Material :type Upgrade%20Material%20Object%20Reference))
  (CallFunction|AddItemtoInventory Material))

(event Custom|Multicast%20Detach%20Cable%20from%20Player)

(event Custom|Multicast%20Attach%20Cable%20To%20Player
  (params (Actor :type Actor%20Object%20Reference))
  (Class|CableComponent|SetAttachEndto (Variables|Default|GetCable) Actor "None" "None"))

(event Custom|Multicast%20Add%20Item%20to%20Inventory
  (params (Material :type Upgrade%20Material%20Object%20Reference))
  (CallFunction|IncreaseMassandSize))

(event EventBeginPlay)

(event Collision|EventActorBeginOverlap
  (params (OtherActor :type Actor%20Object%20Reference)))

(event EventTick
  (params (DeltaSeconds :type Float%20%28single-precision%29)))

(fn ConstructionScript)

(fn OnRepInventory)

(fn OnRepWoodCount)

(fn OnRepMetalCount)

(fn OnRepGearCount)

(fn AddItemtoInventory
  (params (Material :type Upgrade%20Material%20Object%20Reference))
  (Utilities|Casting|CastToLog Material
    (:then
      (bind _result (Math|Integer|IncrementInt (Variables|Inventory|GetWood%20Count))
        (:%20%20
          (Variables|Inventory|SetWood%20Count _result))))
    (:CastFailed
      _))
  (CallFunction|MulticastAddItemtoInventory Material)
  (return))

(fn CreateLeash
  (params (Leasher :type Third%20Person%20Character%20Object%20Reference))
  (bind _returnvalue (Game|SpawnActorfromClass "/Game/Blueprints/Leash.Leash_C" (Transformation|GetActorTransform) "Undefined" Leasher 0))
  (bind _output_get (Variables|Default|SetLeash _returnvalue))
  (Class|PhysicsConstraintComponent|SetConstrainedComponents (Variables|/Script/Engine.PhysicsConstraintActor|GetConstraintComp _output_get) (Variables|Default|GetStaticMesh) "None" (Variables|/Script/Engine.Character|GetCapsuleComponent Leasher) "None")
  (CallFunction|MulticastAttachCabletoPlayer Leasher)
  (return))

(fn OnRepLeash)

(fn IncreaseMassandSize
  (bind _total_resources (CallFunction|GetTotalResourceCount))
  (Class|PrimitiveComponent|SetMassOverrideinKg (Variables|Default|GetStaticMesh) "None" (Math|Conversions|ToFloat(Integer) (* _total_resources 420)) true)
  (Development|PrintString (Utilities|String|ToString(Vector) (* "1.000000,1.000000,1.000000" (Math|Integer|Max(Integer) (/ _total_resources 5) 1))))
  (Transformation|SetActorScale3D (* "1.000000,1.000000,1.000000" (Math|Integer|Max(Integer) (/ _total_resources 5) 1))))

(fn GetTotalResourceCount
  (return (+ (Variables|Inventory|GetWood%20Count) (Variables|Inventory|GetMetal%20Count) (Variables|Inventory|GetGear%20Count))))

(fn RemoveItemsfromInventory
  (params (Amount :type Integer))
  (if (>= (Variables|Inventory|GetWood%20Count) Amount)
    (bind _output_get (Variables|Inventory|SetWood%20Count (- (Variables|Inventory|GetWood%20Count) Amount)))
    (if (<= _output_get 0)
      (Actor|DestroyActor))
    (return true)
    (else
      (return false))))