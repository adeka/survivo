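; Destroyable actor that takes a set number of hits, then spawns its material drops and destroys itself.
; TakeDamage runs only on authority, spawning an impact emitter, triggering a shake and incrementing the hit count.
; Tick polls that count and scatters each DropMats class at a random horizontal offset.
; The shake timeline randomly jitters mesh rotation, then restores the rotation cached in the construction script.
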(event Custom|Shake
  ;[1 1 1] Shake Impact Event Animation
  (Timeline|Timeline_0 PlayFromStart
    (:Update
      (Transformation|AddRelativeRotation (Variables|Default|Getmesh) (Math|Rotator|MakeRotator (Math|Random|RandomFloatinRange -0.3 0.3) (Math|Random|RandomFloatinRange -0.3 0.3) 0.0) false false))
    (:Finished
      (Transformation|SetRelativeRotation (Variables|Default|Getmesh) (Variables|Default|GetOriginalRotation) false false))))

(event Custom|Server%20Spawn%20Particles
  ;[1 1 1] Server Spawn Particles
  (CallFunction|SpawnParticles))

(event Collision|EventActorBeginOverlap
  (params (OtherActor :type Actor%20Object%20Reference))
  (|CallParentFunction OtherActor))

(event EventTick
  (params (DeltaSeconds :type Float%20%28single-precision%29))
  (bind _returnvalue (Transformation|GetActorTransform))
  (bind (_location _rotation _scale) (Math|Transform|BreakTransform _returnvalue))
  ;[1 1 1] Destroy if enough hits are taken
  (if (and (>= (Variables|Default|GetHits) (Variables|Default|GetMaxHits)) (not (Variables|Default|GetDestroyed)))
    (Variables|Default|SetDestroyed true)
    (for _array_element (Variables|Default|GetDropMats)
      (Game|SpawnActorfromClass _array_element (Math|Transform|MakeTransform (+ _location (Math|Vector|MakeVector (Math|Random|RandomFloatinRange -1e+02 1e+02) (Math|Random|RandomFloatinRange -1e+02 1e+02) 0.0)) _rotation _scale) "Undefined" 0 0))
    (Actor|DestroyActor)))

(fn ConstructionScript
  (|CallParentFunction)
  (Variables|Default|SetOriginalRotation (.Rotation (Math|Transform|BreakTransform (Transformation|GetRelativeTransform (Variables|Default|Getmesh))))))

(fn TakeDamage
  (Networking|SwitchHasAuthority
    (:Authority
      (CallFunction|ServerSpawnParticles)
      (CallFunction|Shake)
      (Math|Integer|IncrementInt (Variables|Default|GetHits)))))

(fn SpawnParticles
  (Effects|SpawnEmitteratLocation "/Game/ParticleFX/Impact.Impact" (+ (.Location (Math|Transform|BreakTransform (Transformation|GetActorTransform self))) "0, 0,100.000000"))
  (return))