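; Consumable item actor that a character can eat, passing a fixed amount to that character's Eat function.
; The Eat event checks for authority and only on that side forwards the character to ServerEat.
; ServerEat applies the effect to the character and then destroys the item, while the default BeginPlay, overlap and Tick events remain unused.
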(event Custom|Server%20Eat
  (params (character :type Third%20Person%20Character%20Object%20Reference))
  (Default|Eat character 25.0)
  (Actor|DestroyActor))

(event Custom|Eat
  (params (character :type Third%20Person%20Character%20Object%20Reference))
  (Networking|SwitchHasAuthority
    (:Authority
      (CallFunction|ServerEat character))))

(event EventBeginPlay
  (|CallParentFunction))

(event Collision|EventActorBeginOverlap
  (params (OtherActor :type Actor%20Object%20Reference))
  (|CallParentFunction OtherActor))

(event EventTick
  (params (DeltaSeconds :type Float%20%28single-precision%29))
  (|CallParentFunction DeltaSeconds))

(fn ConstructionScript
  (|CallParentFunction))