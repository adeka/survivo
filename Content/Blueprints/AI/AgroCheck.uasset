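; AgroCheck is a behavior tree tick node that finds visible targets around the pawn of a Follower_AI_Controller.
; Each tick, a multi-sphere object trace gathers nearby candidates, ignoring every AI_Character.
; A Camera-channel line trace tests sight to each, setting TargetToFollow and TargetLocation when clear, or clearing only TargetToFollow when blocked.
; Every hit overwrites the blackboard, so the last one processed wins, and zero hits leave it unchanged.
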(event EventReceiveTickAI
  (params (OwnerController :type AI%20Controller%20Object%20Reference) (ControlledPawn :type Pawn%20Object%20Reference) (DeltaSeconds :type Float%20%28single-precision%29))
  (Utilities|IsValid (Variables|Default|GetController)
    (:Is%20Valid
      _)
    (:Is%20Not%20Valid
      (bind _asfollower_ai_controller (Utilities|Casting|CastToFollower_AI_Controller OwnerController))
      (Variables|Default|SetController _asfollower_ai_controller)))
  (bind _outactors (Actor|GetAllActorsOfClass "/Game/Blueprints/AI/AI_Character.AI_Character_C"))
  (bind _output_get (Variables|Default|SetMy%20Location (Transformation|GetActorLocation (Pawn|GetControlledPawn (Variables|Default|GetController)))))
  (bind _output_get_2 (Variables|Default|SetActors%20to%20Ignore _outactors))
  (bind _outhits (Collision|MultiSphereTraceForObjects _output_get (+ (Transformation|GetActorLocation (Pawn|GetControlledPawn (Variables|Default|GetController))) "0, 0,15.000000") 1.5e+03 (Variables|Default|GetDesired%20Object%20Type) false _output_get_2 "None"))
  (bind _array_element (Utilities|Array|ForEachLoopwithBreak _outhits)
    (:LoopBody
      (bind _outhit (Collision|LineTraceByChannel (Variables|Default|GetMy%20Location) (Transformation|GetActorLocation (.HitActor (Collision|BreakHitResult _array_element))) "TraceTypeQuery2" false (Variables|Default|GetActors%20to%20Ignore) "None"))
      (if (== (.HitActor (Collision|BreakHitResult _outhit)) (.HitActor (Collision|BreakHitResult _array_element)))
        (Class|BTFunctionLibrary|SetBlackboardValueasObject (Variables|Default|GetTarget%20to%20Follow) (.HitActor (Collision|BreakHitResult _outhit)))
        (AI|BehaviorTree|SetBlackboardValueasVector (Variables|Default|GetTarget%20Location) (Transformation|GetActorLocation (.HitActor (Collision|BreakHitResult _outhit))))
        (else
          (Class|BTFunctionLibrary|SetBlackboardValueasObject (Variables|Default|GetTarget%20to%20Follow)))))))