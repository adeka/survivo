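; PoleStand is a usable placeholder that lets a player found a clan and claim its House.
; Using it takes items from the player's leashed bag and, on success, shows the flag setup HUD.
; ServerSetupFlagandHouse runs SetupFlagAndHouse without forwarding a passcode, setting the clan on character and House.
; Setup also hands the loot bag to the House, closes doors, spawns stations, and replaces the stand with a FlagPole.
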(event Custom|Server%20Setup%20Flag%20and%20House
  (params (Owner :type Actor%20Object%20Reference) (Character :type Third%20Person%20Character%20Object%20Reference) (Flag%20Text :type String))
  (Development|PrintString "Hello")
  (CallFunction|SetupFlagandHouse Owner Character Flag%20Text))

(event EventTriggerUse
  (params (User :type Third%20Person%20Character%20Object%20Reference))
  (bind _leashedbag (Variables|/Game/Blueprints/Characters/ThirdPersonCharacter.ThirdPersonCharacter_C|GetLeashedBag User))
  ;[1 1 1] we do need to show a menu for this at some point
  (bind _assurvivo_player_controller (Utilities|Casting|CastToSurvivoPlayerController (Pawn|GetController User)))
  (Utilities|IsValid _leashedbag
    (:Is%20Valid
      (bind _success (Default|RemoveItemsfromInventory _leashedbag 5))
      (if _success
        (Default|OwnerShowSetupFlagHUD _assurvivo_player_controller self)))))

(fn ConstructionScript)

(fn OnRepHouse)

(fn SetupFlagandHouse
  (params (Owner :type Actor%20Object%20Reference) (Character :type Third%20Person%20Character%20Object%20Reference) (Flag%20Text :type String) (Passcode :type String))
  (bind _house (Variables|Default|GetHouse))
  (LocalVariables|SetClan%20Name Flag%20Text)
  (LocalVariables|SetLocal%20Passcode Passcode)
  (Default|TakePlayerLootBag (Variables|Default|GetHouse) Character)
  (Game|SpawnActorfromClass "/Game/Blueprints/Buildings/FlagPole.FlagPole_C" (Transformation|GetActorTransform) "Undefined" Owner (LocalVariables|GetClan%20Name) (Variables|Default|GetHouse) 0)
  (Default|SetupClan Character (LocalVariables|GetClan%20Name) (LocalVariables|GetLocal%20Passcode))
  (Default|SetTeam _house (LocalVariables|GetClan%20Name) (LocalVariables|GetLocal%20Passcode))
  (Default|CloseAllDoors _house Character)
  (Default|SpawnStations _house Character)
  (Actor|DestroyActor))