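; FlagPole is a building actor that displays a text label on its flag and carries a player start named after that label.
; On BeginPlay it writes FlagText to four text render components.
; In the same loop it casts the child actor to PlayerStart and sets its PlayerStartTag to the same text.
; FlagText has a RepNotify function, which is empty.
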(event EventBeginPlay
  (CallFunction|SetTextonFlag))

(event Collision|EventActorBeginOverlap
  (params (OtherActor :type Actor%20Object%20Reference)))

(event EventTick
  (params (DeltaSeconds :type Float%20%28single-precision%29)))

(fn ConstructionScript)

(fn SetTextonFlag
  (bind _output_get (LocalVariables|SetAll%20Text%20Renders (Utilities|Array|MakeArray (Variables|Default|GetTextRender) (Variables|Default|GetTextRender1) (Variables|Default|GetTextRender2) (Variables|Default|GetTextRender3))))
  (for _array_element _output_get
    (Rendering|Components|TextRender|SetText _array_element (Utilities|Text|ToText(String) (Variables|Default|GetFlag%20Text)))
    (bind _asplayer_start (Utilities|Casting|CastToPlayerStart (Variables|/Script/Engine.ChildActorComponent|GetChildActor (Variables|Default|GetChildActor))))
    (Variables|/Script/Engine.PlayerStart|SetPlayerStartTag _asplayer_start (Utilities|String|StringToName (Variables|Default|GetFlag%20Text)))))

(fn OnRepFlagText)