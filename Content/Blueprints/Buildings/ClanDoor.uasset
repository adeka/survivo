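; ClanDoor is a buildable door that only opens or closes for players in the matching clan.
; On TriggerUse it casts the user's controller to SurvivoPlayerController and compares its clan name to the door's ClanName.
; A match flips Open and plays a timeline forward or in reverse to drive the static mesh's yaw.
; Open and ClanName have RepNotify functions, but these and ToggleOpen are empty.
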(event EventBeginPlay)

(event EventTriggerUse
  (params (User :type Third%20Person%20Character%20Object%20Reference))
  (bind _assurvivo_player_controller (Utilities|Casting|CastToSurvivoPlayerController (Pawn|GetController User)))
  (if (Utilities|Enum|Equal(Enum) (Variables|/Game/Blueprints/Gameplay/Clan.Clan_C|GetClan%20Name (Variables|/Game/Blueprints/Gameplay/SurvivoPlayerController.SurvivoPlayerController_C|GetClan _assurvivo_player_controller)) (Variables|Door|GetClan%20Name))
    (if (not (Variables|Door|GetOpen))
      (Variables|Door|SetOpen true)
      (bind _newtrack_0 (Timeline|Timeline_0 PlayFromStart)
        (:Update
          (Transformation|SetRelativeRotation (Variables|Default|GetStaticMesh) (Math|Rotator|MakeRotator 0.0 0.0 _newtrack_0) false false)))
      (else
        (Variables|Door|SetOpen false)
        (Timeline|Timeline_0 ReverseFromEnd)))))

(fn ConstructionScript)

(fn OnRepOpen)

(fn OnRepClanName)

(fn ToggleOpen)