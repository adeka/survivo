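; Utility Blueprint with one function that tests whether an actor faces a target actor.
; It takes the arccosine of the normalized dot product between the actor's forward vector and the offset from target to actor.
; NormalizeToRange remaps that angle so the result is true at 90 degrees or more, meaning the target lies in the actor's front hemisphere.
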(fn ActorFacingOtherActor
  (params (Actor :type Actor%20Object%20Reference) (Target%20Actor :type Actor%20Object%20Reference))
  (bind _returnvalue (Transformation|GetActorForwardVector Actor))
  (bind _returnvalue_2 (Transformation|GetActorLocation Actor))
  (bind _returnvalue_3 (Transformation|GetActorLocation Target%20Actor))
  (bind _returnvalue_4 (- _returnvalue_2 _returnvalue_3))
  (return (>= (Math|Float|NormalizetoRange (Class|KismetMathLibrary|DegAcos (/ (/ (Math|Vector|DotProduct _returnvalue _returnvalue_4) (Math|Vector|VectorLength _returnvalue)) (Math|Vector|VectorLength _returnvalue_4))) -9e+01 9e+01) 1.0)))