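; Door actor that swings open or closed each time its TriggerUse event fires.
; An Open flag picks between playing a timeline from the start and reversing it from the end, with the timeline track driving the Door component's relative yaw.
; Because each toggle restarts from an endpoint, a mid-swing toggle jumps rather than continuing from the current angle.
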(event EventBeginPlay)

(event Collision|EventActorBeginOverlap
  (params (OtherActor :type Actor%20Object%20Reference))
  (|CallParentFunction OtherActor) ; This node is disabled and will not be called.\nDrag off pins to build functionality.
)

(event EventTriggerUse
  (params (character :type Third%20Person%20Character%20Object%20Reference))
  ;[1 1 1] Toogle Door Open / Closed
  (if (Variables|Default|GetOpen)
    (Variables|Default|SetOpen false)
    (bind _newtrack_0 (Timeline|Timeline_0 ReverseFromEnd)
      (:Update
        (Transformation|SetRelativeRotation (Variables|Default|Getdoor) (Math|Rotator|MakeRotator 0.0 0.0 _newtrack_0) false false)))
    (else
      (Variables|Default|SetOpen true)
      (Timeline|Timeline_0 PlayFromStart))))

(fn ConstructionScript
  (|CallParentFunction))